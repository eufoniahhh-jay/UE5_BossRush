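; BP_Boss_Steel is a melee boss character that fights the player with parryable slashes and an unblockable red attack.
; A looping timer picks a random close-range pattern, or at mid range favors a launched dash slash over AI chasing.
; Montage attacks set damage and parry flags, with a sphere trace applying hits.
; Incoming damage feeds health and posture; stun interrupts attacks, and death notifies BP_StageManager.
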(event Custom|TryAttackPlayer
  (bind _returnvalue (Transformation|GetActorLocation))
  (bind _targetplayer (Variables|Default|GetTargetPlayer))
  (bind _returnvalue_2 (Transformation|GetActorLocation _targetplayer))
  (bind _returnvalue_3 (Math|Vector|Distance(Vector) _returnvalue _returnvalue_2))
  (if (Variables|Default|GetbCanAct)
    (if (not (Class|BossBase|IsDead))
      (if (not (Class|BossBase|IsStunned))
        (if (not (Variables|Default|GetbIsAttacking))
          (Utilities|IsValid _targetplayer
            (:Is%20Valid
              (if (<= _returnvalue_3 (Variables|Default|GetAttackRange))
                (AI|Navigation|StopMovement (Pawn|GetController))
                (bind _newparam (CallFunction|SelectAttackPattern))
                (Variables|Default|SetCurrentPattern _newparam)
                (switch Utilities|FlowControl|Switch|SwitchonE_BossAttackPattern (Variables|Default|GetCurrentPattern)
                  (:NewEnumerator0
                    (CallFunction|StartBasicSlash))
                  (:NewEnumerator1
                    (CallFunction|StartDoubleSlash))
                  (:NewEnumerator2
                    (CallFunction|StartRedUnblockable)))
                (elif (and (>= _returnvalue_3 (Variables|DashSlash|GetDashSlashMinDistance)) (<= _returnvalue_3 (Variables|DashSlash|GetDashSlashMaxDistance)))
                  (if (< (Math|Random|RandomIntegerinRange 0 99) 70)
                    (bind _output_get (Variables|Default|SetCurrentPattern "NewEnumerator3"))
                    (switch Utilities|FlowControl|Switch|SwitchonE_BossAttackPattern _output_get
                      (:NewEnumerator3
                        (CallFunction|StartDashSlash)))
                    (else
                      (AI|AIMoveTo self "0, 0, 0" (Variables|Default|GetTargetPlayer) (Variables|Default|GetMoveAcceptanceRadius) false)))
                  (else
                    (AI|AIMoveTo self "0, 0, 0" (Variables|Default|GetTargetPlayer) (Variables|Default|GetMoveAcceptanceRadius) false)))))))))))

(event Custom|StartBasicSlash
  (Development|PrintString "Pattern: Basic Slash")
  (Variables|Default|SetbIsAttacking true)
  (Variables|Default|SetbCurrentAttackParryable true)
  (Variables|Default|SetBossAttackDamage (Variables|Default|GetBasicSlashDamage))
  (Transformation|SetActorRotation (Math|Rotator|MakeRotator 0.0 0.0 (.Yaw (Math|Rotator|BreakRotator (Math|Rotator|FindLookatRotation (Transformation|GetActorLocation) (Transformation|GetActorLocation (Variables|Default|GetTargetPlayer)))))))
  (Animation|PlayAnimMontage "/Game/Blueprints/Boss/AM_PrimaryAttack_RA.AM_PrimaryAttack_RA" 1.0 "None"))

(event Custom|StartDoubleSlash
  (bind _returnvalue (Transformation|GetActorLocation))
  (bind _targetplayer (Variables|Default|GetTargetPlayer))
  (bind _returnvalue_2 (Transformation|GetActorLocation _targetplayer))
  (bind _returnvalue_3 (Math|Rotator|FindLookatRotation _returnvalue _returnvalue_2))
  (bind _yaw (Math|Rotator|BreakRotator _returnvalue_3))
  (bind _returnvalue_4 (Math|Rotator|MakeRotator 0.0 0.0 _yaw))
  (Development|PrintString "Pattern: Double Slash")
  (Variables|Default|SetbIsAttacking true)
  (Variables|Default|SetbIsComboPattern true)
  (Variables|Default|SetbCurrentAttackParryable true)
  (Variables|Default|SetBossAttackDamage (Variables|Default|GetDoubleSlashDamage))
  (Transformation|SetActorRotation _returnvalue_4)
  (Animation|PlayAnimMontage "/Game/Blueprints/Boss/AM_PrimaryAttack_RA.AM_PrimaryAttack_RA" 1.0 "None")
  (Utilities|FlowControl|Delay (Variables|Default|GetComboSecondAttackDelay))
  (if (not (Variables|Default|GetbIsStunned))
    (Development|PrintString "Pattern: Double Slash 2")
    (Transformation|SetActorRotation _returnvalue_4)
    (Animation|PlayAnimMontage (Variables|Default|GetDoubleSlashSecondMontage) 1.0 "None")
    (Utilities|FlowControl|Delay 1.0)
    (Variables|Default|SetbIsComboPattern false)
    (Variables|Default|SetbIsAttacking false)
    (Development|PrintString "Double Slash End")))

(event Custom|StartRedUnblockable
  (Development|PrintString "Pattern: Red Unblockable")
  (Variables|Default|SetbIsAttacking true)
  (Variables|Default|SetbIsComboPattern false)
  (Variables|Default|SetbCurrentAttackParryable false)
  (Variables|Default|SetBossAttackDamage (Variables|Default|GetRedUnblockableDamage))
  (Development|PrintString "RED ATTACK!")
  (Rendering|Components|Light|SetIntensity (Variables|Default|GetRedAttackWarningLight) 8e+03)
  (Utilities|FlowControl|Delay (Variables|Default|GetRedAttackWarningTime))
  (Rendering|Components|Light|SetIntensity (Variables|Default|GetRedAttackWarningLight) 0.0)
  (Transformation|SetActorRotation (Math|Rotator|MakeRotator 0.0 0.0 (.Yaw (Math|Rotator|BreakRotator (Math|Rotator|FindLookatRotation (Transformation|GetActorLocation) (Transformation|GetActorLocation (Variables|Default|GetTargetPlayer)))))))
  (Animation|PlayAnimMontage (Variables|Default|GetRedUnblockableMontage) 1.0 "None"))

(event Custom|StopBossBattle
  (Variables|Default|SetbCanAct false)
  (Variables|Default|SetbIsAttacking false)
  (Variables|Default|SetbIsComboPattern false)
  (Variables|Default|SetbCurrentAttackParryable false)
  (Animation|Montage|MontageStop (Components|SkeletalMesh|GetAnimInstance (Variables|Character|GetMesh)) 0.1 0))

(event Custom|StartDashSlash
  (bind _returnvalue (Transformation|GetActorForwardVector))
  (bind _dashslashmovespeed (Variables|DashSlash|GetDashSlashMoveSpeed))
  (bind _returnvalue_2 (* _returnvalue _dashslashmovespeed))
  (bind (_x _y) (Math|Vector|BreakVector _returnvalue_2))
  (Development|PrintString "Pattern: Dash Slash")
  (AI|Navigation|StopMovement (Pawn|GetController))
  (Components|Movement|StopMovementImmediately (Variables|Character|GetCharacterMovement))
  (Variables|Default|SetbIsAttacking true)
  (Variables|Default|SetbIsComboPattern false)
  (Variables|DashSlash|SetbIsDashing true)
  (Variables|Default|SetbCurrentAttackParryable true)
  (Variables|Default|SetBossAttackDamage (Variables|DashSlash|GetDashSlashDamage))
  (Transformation|SetActorRotation (Math|Rotator|MakeRotator 0.0 0.0 (.Yaw (Math|Rotator|BreakRotator (Math|Rotator|FindLookatRotation (Transformation|GetActorLocation) (Transformation|GetActorLocation (Variables|Default|GetTargetPlayer)))))))
  (Utilities|FlowControl|Delay (Variables|DashSlash|GetDashSlashWindUpTime))
  (if (not (Class|BossBase|IsDead))
    (if (not (Class|BossBase|IsStunned))
      (if (Variables|Default|GetbCanAct)
        (Animation|PlayAnimMontage (Variables|Default|GetDashSlashMontage) 1.0 "None")
        (Character|LaunchCharacter (Math|Vector|MakeVector _x _y 0.0) true false)
        (Utilities|FlowControl|Delay (Variables|DashSlash|GetDashSlashMoveDuration))
        (Variables|DashSlash|SetbIsDashing false)
        (Components|Movement|StopMovementImmediately (Variables|Character|GetCharacterMovement))
        (Utilities|FlowControl|Delay (Variables|DashSlash|GetDashSlashRecoveryTime))
        (Variables|Default|SetbIsAttacking false)
        (Variables|Default|SetbCurrentAttackParryable false)))))

(event EventBeginPlay
  (Variables|Default|SetbCanAct false)
  (Utilities|FlowControl|Delay 3.0)
  (Variables|Default|SetbCanAct true)
  (Variables|Default|SetTargetPlayer (Game|GetPlayerCharacter 0))
  (Utilities|Time|SetTimerbyEvent (delegate Custom|TryAttackPlayer) (Variables|Default|GetAttackCheckInterval) true))

(event Collision|EventActorBeginOverlap
  (params (OtherActor :type Actor%20Object%20Reference)))

(event EventTick
  (params (DeltaSeconds :type Float%20%28single-precision%29)))

(event Game|Damage|EventAnyDamage
  (params (Damage :type Float%20%28single-precision%29) (DamageType :type Damage%20Type%20Object%20Reference) (InstigatedBy :type Controller%20Object%20Reference) (DamageCauser :type Actor%20Object%20Reference))
  (Class|BossBase|ApplyBossDamage Damage (Variables|Default|GetBasicAttackPostureDamage)))

(event EventOnBossStunned
  (Variables|Default|SetbIsAttacking false)
  (Variables|Default|SetbIsComboPattern false)
  (Animation|StopAnimMontage 0)
  (Development|PrintString "BOSS STUNNED!"))

(event EventOnBossStunEnded
  (Development|PrintString "BOSS STUN END"))

(event EventOnBossDead
  (bind _returnvalue (Pawn|GetController))
  (Variables|Default|SetbIsAttacking false)
  (Variables|Default|SetbIsComboPattern false)
  (Utilities|IsValid _returnvalue
    (:Is%20Valid
      (AI|Navigation|StopMovement _returnvalue)
      (Components|Movement|StopMovementImmediately (Variables|Character|GetCharacterMovement))
      (Components|Animation|PlayAnimation (Variables|Character|GetMesh) (Variables|Default|GetDeathAnimation) false)
      (Utilities|FlowControl|Delay (Variables|Default|GetDeathAnimDelay))
      (Development|PrintString "BOSS Dead!")
      (bind _returnvalue_2 (Actor|GetActorOfClass "/Game/Blueprints/Managers/BP_StageManager.BP_StageManager_C"))
      (bind _asbp_stage_manager (Utilities|Casting|CastToBP_StageManager _returnvalue_2))
      (Default|OnBossDefeated _asbp_stage_manager))))

(fn ConstructionScript)

(fn HandleBossAttackStart
  (bind _returnvalue (Transformation|GetActorLocation))
  (bind _returnvalue_2 (Math|Vector|MakeVector 0.0 0.0 6e+01))
  (bind _targetplayer (Variables|Default|GetTargetPlayer))
  (bind _returnvalue_3 (+ _returnvalue _returnvalue_2))
  (if (not (Variables|Default|GetbIsDead))
    (if (not (Variables|Default|GetbIsStunned))
      (Development|PrintString "BP HandleBossAttackStart")
      (bind _outhit (Collision|SphereTraceForObjects _returnvalue_3 (+ _returnvalue_3 (* (Transformation|GetActorForwardVector) (Variables|Default|GetBossAttackTraceDistance))) (Variables|Default|GetBossAttackTraceRadius) (Utilities|Array|MakeArray "ObjectTypeQuery3") false (Utilities|Array|MakeArray self) "ForDuration"))
      (if true
        (Development|PrintString (Utilities|String|ToString(Text) (Utilities|Text|FormatText "Boss Trace Hit Actor: {HitActorName}" (Utilities|GetDisplayName (.HitActor (Collision|BreakHitResult _outhit))))))
        (Utilities|IsValid (.HitActor (Collision|BreakHitResult _outhit))
          (:Is%20Valid
            (if (== (.HitActor (Collision|BreakHitResult _outhit)) _targetplayer)
              (Game|Damage|ApplyDamage _targetplayer (Variables|Default|GetBossAttackDamage) (Pawn|GetController) self)
              (Development|PrintString "Boss Hit Player")
              (else
                (Development|PrintString "Boss Hit Actor But Not TargetPlayer"))))
          (:Is%20Not%20Valid
            (Development|PrintString "Boss Trace Hit But Actor Is Invalid")))
        (else
          (Development|PrintString "Boss Attack Missed"))))))

(fn HandleBossAttackEnd
  (Development|PrintString "BP HandleBossAttackEnd")
  (if (Variables|Default|GetbIsComboPattern)
    (Development|PrintString "Combo pattern continues")
    (else
      (Variables|Default|SetbIsAttacking false)
      (Development|PrintString "Boss Attack End"))))

(fn SelectAttackPattern
  (switch int (Math|Random|RandomIntegerinRange 0 2)
    (:0
      (return "NewEnumerator0"))
    (:1
      (return "NewEnumerator1"))
    (:2
      (return "NewEnumerator2"))))