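; BP_BossDummy is a melee boss test dummy with health, death and debug prints.
; A looping timer checks player range and randomly picks Basic Slash, Double Slash or a delayed, unparryable red attack, all reusing one montage.
; HandleBossAttackStart sphere-traces forward to damage the player, and HandleBossAttackEnd clears the attacking state outside combos.
; Damage arrives through AnyDamage or ApplyBossDamage, though only AnyDamage sets IsDead.
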(event Custom|TryAttackPlayer
  (bind _targetplayer (Variables|Default|GetTargetPlayer))
  (if (not (Variables|Default|GetbIsDead))
    (if (not (Variables|Default|GetbIsAttacking))
      (Utilities|IsValid _targetplayer
        (:Is%20Valid
          (if (<= (Math|Vector|Distance(Vector) (Transformation|GetActorLocation) (Transformation|GetActorLocation _targetplayer)) (Variables|Default|GetAttackRange))
            (bind _newparam (CallFunction|SelectAttackPattern))
            (Variables|Default|SetCurrentPattern _newparam)
            (switch Utilities|FlowControl|Switch|SwitchonE_BossAttackPattern (Variables|Default|GetCurrentPattern)
              (:NewEnumerator0
                (CallFunction|StartBasicSlash))
              (:NewEnumerator1
                (CallFunction|StartDoubleSlash))
              (:NewEnumerator2
                (CallFunction|StartRedUnblockable)))))))))

(event Custom|StartBasicSlash
  (Development|PrintString "Pattern: Basic Slash")
  (Variables|Default|SetbIsAttacking true)
  (Variables|Default|SetbCurrentAttackParryable true)
  (Transformation|SetActorRotation (Math|Rotator|MakeRotator 0.0 0.0 (.Yaw (Math|Rotator|BreakRotator (Math|Rotator|FindLookatRotation (Transformation|GetActorLocation) (Transformation|GetActorLocation (Variables|Default|GetTargetPlayer)))))))
  (Animation|PlayAnimMontage "/Game/Blueprints/Boss/AM_PrimaryAttack_RA.AM_PrimaryAttack_RA" 1.0 "None"))

(event Custom|StartDoubleSlash
  (bind _returnvalue (Transformation|GetActorLocation))
  (bind _targetplayer (Variables|Default|GetTargetPlayer))
  (bind _returnvalue_2 (Transformation|GetActorLocation _targetplayer))
  (bind _returnvalue_3 (Math|Rotator|FindLookatRotation _returnvalue _returnvalue_2))
  (bind _yaw (Math|Rotator|BreakRotator _returnvalue_3))
  (bind _returnvalue_4 (Math|Rotator|MakeRotator 0.0 0.0 _yaw))
  (Development|PrintString "Pattern: Double Slash")
  (Variables|Default|SetbIsAttacking true)
  (Variables|Default|SetbIsComboPattern true)
  (Variables|Default|SetbCurrentAttackParryable true)
  (Transformation|SetActorRotation _returnvalue_4)
  (Animation|PlayAnimMontage "/Game/Blueprints/Boss/AM_PrimaryAttack_RA.AM_PrimaryAttack_RA" 1.0 "None")
  (Utilities|FlowControl|Delay (Variables|Default|GetComboSecondAttackDelay))
  (Development|PrintString "Pattern: Double Slash 2")
  (Transformation|SetActorRotation _returnvalue_4)
  (Animation|PlayAnimMontage "/Game/Blueprints/Boss/AM_PrimaryAttack_RA.AM_PrimaryAttack_RA" 1.0 "None")
  (Utilities|FlowControl|Delay 1.0)
  (Variables|Default|SetbIsComboPattern false)
  (Variables|Default|SetbIsAttacking false)
  (Development|PrintString "Double Slash End"))

(event Custom|StartRedUnblockable
  (Development|PrintString "Pattern: Red Unblockable")
  (Variables|Default|SetbIsAttacking true)
  (Variables|Default|SetbIsComboPattern false)
  (Variables|Default|SetbCurrentAttackParryable false)
  (Development|PrintString "RED ATTACK!")
  (Utilities|FlowControl|Delay (Variables|Default|GetRedAttackWarningTime))
  (Transformation|SetActorRotation (Math|Rotator|MakeRotator 0.0 0.0 (.Yaw (Math|Rotator|BreakRotator (Math|Rotator|FindLookatRotation (Transformation|GetActorLocation) (Transformation|GetActorLocation (Variables|Default|GetTargetPlayer)))))))
  (Animation|PlayAnimMontage "/Game/Blueprints/Boss/AM_PrimaryAttack_RA.AM_PrimaryAttack_RA" 1.0 "None"))

(event EventBeginPlay
  (Variables|Default|SetCurrentHP (Variables|Default|GetMaxHP))
  (Variables|Default|SetbIsDead false)
  (Variables|Default|SetTargetPlayer (Game|GetPlayerCharacter 0))
  (Utilities|Time|SetTimerbyEvent (delegate Custom|TryAttackPlayer) (Variables|Default|GetAttackCheckInterval) true))

(event Collision|EventActorBeginOverlap
  (params (OtherActor :type Actor%20Object%20Reference)))

(event EventTick
  (params (DeltaSeconds :type Float%20%28single-precision%29)))

(event Game|Damage|EventAnyDamage
  (params (Damage :type Float%20%28single-precision%29) (DamageType :type Damage%20Type%20Object%20Reference) (InstigatedBy :type Controller%20Object%20Reference) (DamageCauser :type Actor%20Object%20Reference))
  (if (not (Variables|Default|GetbIsDead))
    (bind _output_get (Variables|Default|SetCurrentHP (Math|Float|Clamp(Float) (- (Variables|Default|GetCurrentHP) Damage) 0.0 (Variables|Default|GetMaxHP))))
    (Development|PrintString (Utilities|String|ToString(Text) (Utilities|Text|FormatText "Boss HP: {HP}" _output_get)))
    (if (<= (Variables|Default|GetCurrentHP) 0.0)
      (Variables|Default|SetbIsDead true)
      (Development|PrintString "Boss Dead"))))

(fn ConstructionScript)

(fn ApplyBossDamage
  (params (DamageAmount :type Float%20%28double-precision%29))
  (Development|PrintString (Utilities|String|ToString(Float) DamageAmount))
  (bind _output_get (Variables|Default|SetCurrentHP (Math|Float|Clamp(Float) (- (Variables|Default|GetCurrentHP) DamageAmount) 0.0 (Variables|Default|GetMaxHP))))
  (Development|PrintString (Utilities|String|ToString(Text) (Utilities|Text|FormatText "Boss HP: {HP}" _output_get)))
  (if (<= (Variables|Default|GetCurrentHP) 0.0)
    (Development|PrintString "Boss Dead")))

(fn GetCurrentHP
  (return (Variables|Default|GetCurrentHP)))

(fn GetMaxHP
  (return (Variables|Default|GetMaxHP)))

(fn HandleBossAttackStart
  (bind _returnvalue (Transformation|GetActorLocation))
  (bind _returnvalue_2 (Math|Vector|MakeVector 0.0 0.0 6e+01))
  (bind _targetplayer (Variables|Default|GetTargetPlayer))
  (bind _returnvalue_3 (+ _returnvalue _returnvalue_2))
  (Development|PrintString "BP HandleBossAttackStart")
  (bind _outhit (Collision|SphereTraceForObjects _returnvalue_3 (+ _returnvalue_3 (* (Transformation|GetActorForwardVector) (Variables|Default|GetBossAttackTraceDistance))) (Variables|Default|GetBossAttackTraceRadius) (Utilities|Array|MakeArray "ObjectTypeQuery3") false (Utilities|Array|MakeArray self) "ForDuration"))
  (if true
    (Development|PrintString (Utilities|String|ToString(Text) (Utilities|Text|FormatText "Boss Trace Hit Actor: {HitActorName}" (Utilities|GetDisplayName (.HitActor (Collision|BreakHitResult _outhit))))))
    (Utilities|IsValid (.HitActor (Collision|BreakHitResult _outhit))
      (:Is%20Valid
        (if (== (.HitActor (Collision|BreakHitResult _outhit)) _targetplayer)
          (Game|Damage|ApplyDamage _targetplayer (Variables|Default|GetBossAttackDamage) (Pawn|GetController) self)
          (Development|PrintString "Boss Hit Player")
          (else
            (Development|PrintString "Boss Hit Actor But Not TargetPlayer"))))
      (:Is%20Not%20Valid
        (Development|PrintString "Boss Trace Hit But Actor Is Invalid")))
    (else
      (Development|PrintString "Boss Attack Missed"))))

(fn HandleBossAttackEnd
  (Development|PrintString "BP HandleBossAttackEnd")
  (if (Variables|Default|GetbIsComboPattern)
    (Development|PrintString "Combo pattern continues")
    (else
      (Variables|Default|SetbIsAttacking false)
      (Development|PrintString "Boss Attack End"))))

(fn SelectAttackPattern
  (switch int (Math|Random|RandomIntegerinRange 0 2)
    (:0
      (return "NewEnumerator0"))
    (:1
      (return "NewEnumerator1"))
    (:2
      (return "NewEnumerator2"))))