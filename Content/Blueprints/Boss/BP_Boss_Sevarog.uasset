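; Sevarog boss character that chases the player, attacks in range, takes health/posture damage, and reports death to BP_StageManager.
; A looping timer picks weighted random slash, triple strike, slam or shockwave patterns, setting damage and parry flags.
; Montage attacks use delays and HandleBossAttackStart/End for sphere-trace hits, while shockwave damages through a delayed overlap.
; Double slash, red unblockable, backstep and dash slash exist but are outside the selection.
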(event Custom|TryAttackPlayer
  (bind _targetplayer (Variables|Default|GetTargetPlayer))
  (if (Variables|Default|GetbCanAct)
    (if (not (Class|BossBase|IsDead))
      (if (not (Class|BossBase|IsStunned))
        (if (not (Variables|Default|GetbIsAttacking))
          (Utilities|IsValid _targetplayer
            (:Is%20Valid
              (if (<= (Math|Vector|Distance(Vector) (Transformation|GetActorLocation) (Transformation|GetActorLocation _targetplayer)) (Variables|Default|GetAttackRange))
                (AI|Navigation|StopMovement (Pawn|GetController))
                (bind _newparam (CallFunction|SelectAttackPattern))
                (Variables|Default|SetCurrentPattern _newparam)
                (switch Utilities|FlowControl|Switch|SwitchonE_BossAttackPattern (Variables|Default|GetCurrentPattern)
                  (:NewEnumerator0
                    (CallFunction|StartBasicSlash))
                  (:NewEnumerator4
                    (CallFunction|StartTripleStrike))
                  (:NewEnumerator5
                    (CallFunction|StartHeavySlam))
                  (:NewEnumerator6
                    (CallFunction|StartShockwave)))
                (else
                  (AI|AIMoveTo self "0, 0, 0" (Variables|Default|GetTargetPlayer) (Variables|Default|GetMoveAcceptanceRadius) false))))))))))

(event Custom|StartBasicSlash
  (Development|PrintString "Pattern: Basic Slash")
  (Variables|Default|SetbIsAttacking true)
  (Variables|Default|SetbCurrentAttackParryable true)
  (Variables|Default|SetBossAttackDamage (Variables|Default|GetBasicSlashDamage))
  (Transformation|SetActorRotation (Math|Rotator|MakeRotator 0.0 0.0 (.Yaw (Math|Rotator|BreakRotator (Math|Rotator|FindLookatRotation (Transformation|GetActorLocation) (Transformation|GetActorLocation (Variables|Default|GetTargetPlayer)))))))
  (Animation|PlayAnimMontage "/Game/Blueprints/Boss/AM_PrimaryAttack_RA.AM_PrimaryAttack_RA" 1.0 "None")
  (Variables|Default|SetbIsAttacking false))

(event Custom|StartDoubleSlash
  (bind _returnvalue (Transformation|GetActorLocation))
  (bind _targetplayer (Variables|Default|GetTargetPlayer))
  (bind _returnvalue_2 (Transformation|GetActorLocation _targetplayer))
  (bind _returnvalue_3 (Math|Rotator|FindLookatRotation _returnvalue _returnvalue_2))
  (bind _yaw (Math|Rotator|BreakRotator _returnvalue_3))
  (bind _returnvalue_4 (Math|Rotator|MakeRotator 0.0 0.0 _yaw))
  (Development|PrintString "Pattern: Double Slash")
  (Variables|Default|SetbIsAttacking true)
  (Variables|Default|SetbIsComboPattern true)
  (Variables|Default|SetbCurrentAttackParryable true)
  (Variables|Default|SetBossAttackDamage (Variables|Default|GetDoubleSlashDamage))
  (Transformation|SetActorRotation _returnvalue_4)
  (Animation|PlayAnimMontage "/Game/Blueprints/Boss/AM_PrimaryAttack_RA.AM_PrimaryAttack_RA" 1.0 "None")
  (Utilities|FlowControl|Delay (Variables|Default|GetComboSecondAttackDelay))
  (if (not (Variables|Default|GetbIsStunned))
    (Development|PrintString "Pattern: Double Slash 2")
    (Transformation|SetActorRotation _returnvalue_4)
    (Animation|PlayAnimMontage (Variables|Default|GetDoubleSlashSecondMontage) 1.0 "None")
    (Utilities|FlowControl|Delay 1.0)
    (Variables|Default|SetbIsComboPattern false)
    (Variables|Default|SetbIsAttacking false)
    (Development|PrintString "Double Slash End")))

(event Custom|StartRedUnblockable
  (Development|PrintString "Pattern: Red Unblockable")
  (Variables|Default|SetbIsAttacking true)
  (Variables|Default|SetbIsComboPattern false)
  (Variables|Default|SetbCurrentAttackParryable false)
  (Variables|Default|SetBossAttackDamage (Variables|Default|GetRedUnblockableDamage))
  (Development|PrintString "RED ATTACK!")
  (Rendering|Components|Light|SetIntensity (Variables|Default|GetRedAttackWarningLight) 8e+03)
  (Utilities|FlowControl|Delay (Variables|Default|GetRedAttackWarningTime))
  (Rendering|Components|Light|SetIntensity (Variables|Default|GetRedAttackWarningLight) 0.0)
  (Transformation|SetActorRotation (Math|Rotator|MakeRotator 0.0 0.0 (.Yaw (Math|Rotator|BreakRotator (Math|Rotator|FindLookatRotation (Transformation|GetActorLocation) (Transformation|GetActorLocation (Variables|Default|GetTargetPlayer)))))))
  (Animation|PlayAnimMontage (Variables|Default|GetRedUnblockableMontage) 1.0 "None"))

(event Custom|StopBossBattle
  (Variables|Default|SetbCanAct false)
  (Variables|Default|SetbIsAttacking false)
  (Variables|Default|SetbIsComboPattern false)
  (Variables|Default|SetbCurrentAttackParryable false)
  (Animation|Montage|MontageStop (Components|SkeletalMesh|GetAnimInstance (Variables|Character|GetMesh)) 0.1 0))

(event Custom|StartDashSlash
  (bind _returnvalue (Transformation|GetActorForwardVector))
  (bind _dashslashmovespeed (Variables|DashSlash|GetDashSlashMoveSpeed))
  (bind _returnvalue_2 (* _returnvalue _dashslashmovespeed))
  (bind (_x _y) (Math|Vector|BreakVector _returnvalue_2))
  (Development|PrintString "Pattern: Dash Slash")
  (AI|Navigation|StopMovement (Pawn|GetController))
  (Components|Movement|StopMovementImmediately (Variables|Character|GetCharacterMovement))
  (Variables|Default|SetbIsAttacking true)
  (Variables|Default|SetbIsComboPattern false)
  (Variables|DashSlash|SetbIsDashing true)
  (Variables|Default|SetbCurrentAttackParryable true)
  (Variables|Default|SetBossAttackDamage (Variables|DashSlash|GetDashSlashDamage))
  (Transformation|SetActorRotation (Math|Rotator|MakeRotator 0.0 0.0 (.Yaw (Math|Rotator|BreakRotator (Math|Rotator|FindLookatRotation (Transformation|GetActorLocation) (Transformation|GetActorLocation (Variables|Default|GetTargetPlayer)))))))
  (Utilities|FlowControl|Delay (Variables|DashSlash|GetDashSlashWindUpTime))
  (if (not (Class|BossBase|IsDead))
    (if (not (Class|BossBase|IsStunned))
      (if (Variables|Default|GetbCanAct)
        (Animation|PlayAnimMontage (Variables|Default|GetDashSlashMontage) 1.0 "None")
        (Character|LaunchCharacter (Math|Vector|MakeVector _x _y 0.0) true false)
        (Utilities|FlowControl|Delay (Variables|DashSlash|GetDashSlashMoveDuration))
        (Variables|DashSlash|SetbIsDashing false)
        (Components|Movement|StopMovementImmediately (Variables|Character|GetCharacterMovement))
        (Utilities|FlowControl|Delay (Variables|DashSlash|GetDashSlashRecoveryTime))
        (Variables|Default|SetbIsAttacking false)
        (Variables|Default|SetbCurrentAttackParryable false)))))

(event Custom|StartTripleStrike
  (bind _returnvalue (Transformation|GetActorLocation))
  (bind _targetplayer (Variables|Default|GetTargetPlayer))
  (bind _returnvalue_2 (Transformation|GetActorLocation _targetplayer))
  (bind _returnvalue_3 (Math|Rotator|FindLookatRotation _returnvalue _returnvalue_2))
  (bind _yaw (Math|Rotator|BreakRotator _returnvalue_3))
  (bind _returnvalue_4 (Math|Rotator|MakeRotator 0.0 0.0 _yaw))
  (Variables|Default|SetbIsAttacking true)
  (Variables|Default|SetbIsComboPattern true)
  (Variables|Default|SetbCurrentAttackParryable true)
  (Variables|Default|SetBossAttackDamage (Variables|Attack|GetTripleStrikeDamage1))
  (Transformation|SetActorRotation _returnvalue_4)
  (Animation|PlayAnimMontage (Variables|Attack|GetTripleStrikeMontage1) 1.0 "None")
  (Utilities|FlowControl|Delay (Variables|Attack|GetTripleStrikeInterval))
  (if (not (Variables|Default|GetbIsStunned))
    (Transformation|SetActorRotation _returnvalue_4)
    (Animation|PlayAnimMontage (Variables|Attack|GetTripleStrikeMontage2) 1.0 "None")
    (Utilities|FlowControl|Delay (Variables|Attack|GetTripleStrikeInterval))
    (if (not (Variables|Default|GetbIsStunned))
      (Variables|Default|SetBossAttackDamage (Variables|Attack|GetTripleStrikeDamage3))
      (Transformation|SetActorRotation _returnvalue_4)
      (Animation|PlayAnimMontage (Variables|Attack|GetTripleStrikeMontage3) 1.0 "None")
      (Utilities|FlowControl|Delay (Variables|Attack|GetTripleStrikeRecoveryTime))
      (Variables|Default|SetbIsComboPattern false)
      (Variables|Default|SetbIsAttacking false)
      (Development|PrintString "Triple Strike End"))))

(event Custom|StartHeavySlam
  (Variables|Default|SetbIsAttacking true)
  (Variables|Default|SetbIsComboPattern false)
  (Variables|Default|SetbCurrentAttackParryable true)
  (Variables|Default|SetBossAttackDamage (Variables|Default|GetHeavySlamDamage))
  (Utilities|FlowControl|Delay 0.4)
  (Transformation|SetActorRotation (Math|Rotator|MakeRotator 0.0 0.0 (.Yaw (Math|Rotator|BreakRotator (Math|Rotator|FindLookatRotation (Transformation|GetActorLocation) (Transformation|GetActorLocation (Variables|Default|GetTargetPlayer)))))))
  (Animation|PlayAnimMontage (Variables|Default|GetHeavySlamMontage) 1.0 "None")
  (Utilities|FlowControl|Delay 0.2)
  (Variables|Default|SetbIsComboPattern false)
  (Variables|Default|SetbIsAttacking false)
  (Development|PrintString "Heavy Slam End"))

(event Custom|StartShockwave
  (Variables|Default|SetbIsAttacking true)
  (Variables|Default|SetbIsComboPattern false)
  (Variables|Default|SetbCurrentAttackParryable false)
  (Development|PrintString "Dark Explosion Warning")
  (Animation|PlayAnimMontage (Variables|Default|GetShockwaveMontage) 1.0 "None")
  (Rendering|Debug|DrawDebugSphere (Transformation|GetActorLocation) (Variables|Default|GetShockwaveRadius) 24 "(R=1.000000,G=0.001736,B=0.001736,A=1.000000)" 1.0)
  (Camera|PlayWorldCameraShake (Variables|Default|GetShockwaveCameraShake) (Transformation|GetActorLocation) 0.0 1.5e+03)
  (Development|PrintString "Shockwave WindUp")
  (Utilities|FlowControl|Delay (Variables|Default|GetShockwaveWindUpTime))
  (bind _outactors (Collision|SphereOverlapActors (Transformation|GetActorLocation) (Variables|Default|GetShockwaveRadius) (Utilities|Array|MakeArray "ObjectTypeQuery3") "/Game/Blueprints/Player/BP_PlayerCharacter.BP_PlayerCharacter_C" (Utilities|Array|MakeArray self)))
  (for _array_element _outactors
    (Game|Damage|ApplyDamage _array_element (Variables|Default|GetShockwaveDamage) (Pawn|GetController) self))
  (Utilities|FlowControl|Delay (Variables|Default|GetShockwaveRecoveryTime))
  (Variables|Default|SetbIsAttacking false)
  (Variables|Default|SetbIsComboPattern false)
  (Variables|Default|SetbCurrentAttackParryable true))

(event Custom|StartBackstepDash
  (Variables|Default|SetbIsAttacking true)
  (Variables|Default|SetbIsComboPattern false)
  (Variables|Default|SetbCurrentAttackParryable true)
  (Variables|Default|SetBossAttackDamage 0.0)
  (Character|LaunchCharacter (+ (* (Transformation|GetActorForwardVector) (/ (* (Variables|Attack|GetBackstepDistance) -1.0) (Variables|Attack|GetBackstepMoveTime))) (Transformation|GetActorLocation)) true false)
  (Utilities|FlowControl|Delay (Variables|Attack|GetBackstepMoveTime))
  (Components|Movement|StopMovementImmediately (Variables|Character|GetCharacterMovement))
  (Transformation|SetActorRotation (Math|Rotator|MakeRotator 0.0 0.0 (.Yaw (Math|Rotator|BreakRotator (Math|Rotator|FindLookatRotation (Transformation|GetActorLocation) (Transformation|GetActorLocation (Variables|Default|GetTargetPlayer)))))))
  (Utilities|FlowControl|Delay (Variables|Attack|GetBackstepPauseTime))
  (Animation|PlayAnimMontage (Variables|Attack|GetBackstepDashMontage) 1.0 "None")
  (Character|LaunchCharacter (* (Math|Vector|Normalize (- (Transformation|GetActorLocation (Variables|Default|GetTargetPlayer)) (Transformation|GetActorLocation))) (Variables|Attack|GetBackstepDashSpeed)) true false)
  (Utilities|FlowControl|Delay (Variables|Attack|GetBackstepDashDuration))
  (Components|Movement|StopMovementImmediately (Variables|Character|GetCharacterMovement))
  (Utilities|FlowControl|Delay (Variables|Attack|GetBackstepDashRecoveryTime))
  (Variables|Default|SetbIsAttacking false)
  (Variables|Default|SetbIsComboPattern false))

(event EventBeginPlay
  (Variables|Default|SetbCanAct false)
  (Utilities|FlowControl|Delay 3.0)
  (Variables|Default|SetbCanAct true)
  (Variables|Default|SetTargetPlayer (Game|GetPlayerCharacter 0))
  (Utilities|Time|SetTimerbyEvent (delegate Custom|TryAttackPlayer) (Variables|Default|GetAttackCheckInterval) true))

(event Collision|EventActorBeginOverlap
  (params (OtherActor :type Actor%20Object%20Reference)))

(event EventTick
  (params (DeltaSeconds :type Float%20%28single-precision%29)))

(event Game|Damage|EventAnyDamage
  (params (Damage :type Float%20%28single-precision%29) (DamageType :type Damage%20Type%20Object%20Reference) (InstigatedBy :type Controller%20Object%20Reference) (DamageCauser :type Actor%20Object%20Reference))
  (Class|BossBase|ApplyBossDamage Damage (Variables|Default|GetBasicAttackPostureDamage)))

(event EventOnBossStunned
  (Variables|Default|SetbIsAttacking false)
  (Variables|Default|SetbIsComboPattern false)
  (Animation|StopAnimMontage 0)
  (Development|PrintString "BOSS STUNNED!"))

(event EventOnBossStunEnded
  (Development|PrintString "BOSS STUN END"))

(event EventOnBossDead
  (bind _returnvalue (Pawn|GetController))
  (Variables|Default|SetbIsAttacking false)
  (Variables|Default|SetbIsComboPattern false)
  (Utilities|IsValid _returnvalue
    (:Is%20Valid
      (AI|Navigation|StopMovement _returnvalue)
      (Components|Movement|StopMovementImmediately (Variables|Character|GetCharacterMovement))
      (Components|Animation|PlayAnimation (Variables|Character|GetMesh) (Variables|Default|GetDeathAnimation) false)
      (Utilities|FlowControl|Delay (Variables|Default|GetDeathAnimDelay))
      (Development|PrintString "BOSS Dead!")
      (bind _returnvalue_2 (Actor|GetActorOfClass "/Game/Blueprints/Managers/BP_StageManager.BP_StageManager_C"))
      (bind _asbp_stage_manager (Utilities|Casting|CastToBP_StageManager _returnvalue_2))
      (Default|OnBossDefeated _asbp_stage_manager))))

(fn ConstructionScript)

(fn HandleBossAttackStart
  (bind _returnvalue (Transformation|GetActorLocation))
  (bind _returnvalue_2 (Math|Vector|MakeVector 0.0 0.0 6e+01))
  (bind _targetplayer (Variables|Default|GetTargetPlayer))
  (bind _returnvalue_3 (+ _returnvalue _returnvalue_2))
  (if (not (Variables|Default|GetbIsDead))
    (if (not (Variables|Default|GetbIsStunned))
      (Development|PrintString "BP HandleBossAttackStart")
      (if (Utilities|Enum|Equal(Enum) (Variables|Default|GetCurrentPattern) "NewEnumerator5")
        (Camera|PlayWorldCameraShake (Variables|Default|GetHeavyImpactCameraShake) (Transformation|GetActorLocation) 0.0 1.5e+03))
      (bind _outhit (Collision|SphereTraceForObjects _returnvalue_3 (+ _returnvalue_3 (* (Transformation|GetActorForwardVector) (Variables|Default|GetBossAttackTraceDistance))) (Variables|Default|GetBossAttackTraceRadius) (Utilities|Array|MakeArray "ObjectTypeQuery3") false (Utilities|Array|MakeArray self) "ForDuration"))
      (if true
        (Development|PrintString (Utilities|String|ToString(Text) (Utilities|Text|FormatText "Boss Trace Hit Actor: {HitActorName}" (Utilities|GetDisplayName (.HitActor (Collision|BreakHitResult _outhit))))))
        (Utilities|IsValid (.HitActor (Collision|BreakHitResult _outhit))
          (:Is%20Valid
            (if (== (.HitActor (Collision|BreakHitResult _outhit)) _targetplayer)
              (Game|Damage|ApplyDamage _targetplayer (Variables|Default|GetBossAttackDamage) (Pawn|GetController) self)
              (Development|PrintString "Boss Hit Player")
              (else
                (Development|PrintString "Boss Hit Actor But Not TargetPlayer"))))
          (:Is%20Not%20Valid
            (Development|PrintString "Boss Trace Hit But Actor Is Invalid")))
        (else
          (Development|PrintString "Boss Attack Missed"))))))

(fn HandleBossAttackEnd
  (Development|PrintString "BP HandleBossAttackEnd")
  (if (Variables|Default|GetbIsComboPattern)
    (Development|PrintString "Combo pattern continues")
    (else
      (Variables|Default|SetbIsAttacking false)
      (Development|PrintString "Boss Attack End"))))

(fn SelectAttackPattern
  (bind _output_get (LocalVariables|SetRandomPatternValue (Math|Random|RandomFloatinRange 0.0 1e+02)))
  (if (< _output_get 4e+01)
    (Development|PrintString "Sevarog Pattern: Quick Slash")
    (return "NewEnumerator0")
    (elif (< (LocalVariables|GetRandomPatternValue) 65.0)
      (Development|PrintString "Sevarog Pattern: Triple Slash")
      (return "NewEnumerator4")
      (elif (< (LocalVariables|GetRandomPatternValue) 85.0)
        (Development|PrintString "Sevarog Pattern: Heavy Cleave")
        (return "NewEnumerator5")
        (else
          (Development|PrintString "Sevarog Pattern: Dark Explosion")
          (return "NewEnumerator6"))))))