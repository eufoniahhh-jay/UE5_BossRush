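; Grux boss character that fights the player with randomly chosen basic slash, double slash or light-telegraphed unblockable attacks.
; A looping timer chases the player or, in range, starts a montage pattern that sets damage and parryability.
; Attack start/end handlers sphere-trace for damage and release the attack state, except mid-combo.
; Incoming damage feeds HP and posture through ApplyBossDamage, while stun, death and battle-stop events interrupt attacks.
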(event Custom|TryAttackPlayer
  (bind _targetplayer (Variables|Default|GetTargetPlayer))
  (if (Variables|Default|GetbCanAct)
    (if (not (Class|BossBase|IsDead))
      (if (not (Class|BossBase|IsStunned))
        (if (not (Variables|Default|GetbIsAttacking))
          (Utilities|IsValid _targetplayer
            (:Is%20Valid
              (if (<= (Math|Vector|Distance(Vector) (Transformation|GetActorLocation) (Transformation|GetActorLocation _targetplayer)) (Variables|Default|GetAttackRange))
                (AI|Navigation|StopMovement (Pawn|GetController))
                (bind _newparam (CallFunction|SelectAttackPattern))
                (Variables|Default|SetCurrentPattern _newparam)
                (switch Utilities|FlowControl|Switch|SwitchonE_BossAttackPattern (Variables|Default|GetCurrentPattern)
                  (:NewEnumerator0
                    (CallFunction|StartBasicSlash))
                  (:NewEnumerator1
                    (CallFunction|StartDoubleSlash))
                  (:NewEnumerator2
                    (CallFunction|StartRedUnblockable)))
                (else
                  (AI|AIMoveTo self "0, 0, 0" (Variables|Default|GetTargetPlayer) (Variables|Default|GetMoveAcceptanceRadius) false))))))))))

(event Custom|StartBasicSlash
  (Development|PrintString "Pattern: Basic Slash")
  (Variables|Default|SetbIsAttacking true)
  (Variables|Default|SetbCurrentAttackParryable true)
  (Variables|Default|SetBossAttackDamage (Variables|Default|GetBasicSlashDamage))
  (Transformation|SetActorRotation (Math|Rotator|MakeRotator 0.0 0.0 (.Yaw (Math|Rotator|BreakRotator (Math|Rotator|FindLookatRotation (Transformation|GetActorLocation) (Transformation|GetActorLocation (Variables|Default|GetTargetPlayer)))))))
  (Animation|PlayAnimMontage "/Game/Blueprints/Boss/AM_PrimaryAttack_RA.AM_PrimaryAttack_RA" 1.0 "None"))

(event Custom|StartDoubleSlash
  (bind _returnvalue (Transformation|GetActorLocation))
  (bind _targetplayer (Variables|Default|GetTargetPlayer))
  (bind _returnvalue_2 (Transformation|GetActorLocation _targetplayer))
  (bind _returnvalue_3 (Math|Rotator|FindLookatRotation _returnvalue _returnvalue_2))
  (bind _yaw (Math|Rotator|BreakRotator _returnvalue_3))
  (bind _returnvalue_4 (Math|Rotator|MakeRotator 0.0 0.0 _yaw))
  (Development|PrintString "Pattern: Double Slash")
  (Variables|Default|SetbIsAttacking true)
  (Variables|Default|SetbIsComboPattern true)
  (Variables|Default|SetbCurrentAttackParryable true)
  (Variables|Default|SetBossAttackDamage (Variables|Default|GetDoubleSlashDamage))
  (Transformation|SetActorRotation _returnvalue_4)
  (Animation|PlayAnimMontage "/Game/Blueprints/Boss/AM_PrimaryAttack_RA.AM_PrimaryAttack_RA" 1.0 "None")
  (Utilities|FlowControl|Delay (Variables|Default|GetComboSecondAttackDelay))
  (if (not (Variables|Default|GetbIsStunned))
    (Development|PrintString "Pattern: Double Slash 2")
    (Transformation|SetActorRotation _returnvalue_4)
    (Animation|PlayAnimMontage (Variables|Default|GetDoubleSlashSecondMontage) 1.0 "None")
    (Utilities|FlowControl|Delay 1.0)
    (Variables|Default|SetbIsComboPattern false)
    (Variables|Default|SetbIsAttacking false)
    (Development|PrintString "Double Slash End")))

(event Custom|StartRedUnblockable
  (Development|PrintString "Pattern: Red Unblockable")
  (Variables|Default|SetbIsAttacking true)
  (Variables|Default|SetbIsComboPattern false)
  (Variables|Default|SetbCurrentAttackParryable false)
  (Variables|Default|SetBossAttackDamage (Variables|Default|GetRedUnblockableDamage))
  (Development|PrintString "RED ATTACK!")
  (Rendering|Components|Light|SetIntensity (Variables|Default|GetRedAttackWarningLight) 8e+03)
  (Utilities|FlowControl|Delay (Variables|Default|GetRedAttackWarningTime))
  (Rendering|Components|Light|SetIntensity (Variables|Default|GetRedAttackWarningLight) 0.0)
  (Transformation|SetActorRotation (Math|Rotator|MakeRotator 0.0 0.0 (.Yaw (Math|Rotator|BreakRotator (Math|Rotator|FindLookatRotation (Transformation|GetActorLocation) (Transformation|GetActorLocation (Variables|Default|GetTargetPlayer)))))))
  (Animation|PlayAnimMontage (Variables|Default|GetRedUnblockableMontage) 1.0 "None"))

(event Custom|StopBossBattle
  (Variables|Default|SetbCanAct false)
  (Variables|Default|SetbIsAttacking false)
  (Variables|Default|SetbIsComboPattern false)
  (Variables|Default|SetbCurrentAttackParryable false)
  (Animation|Montage|MontageStop (Components|SkeletalMesh|GetAnimInstance (Variables|Character|GetMesh)) 0.1 0))

(event EventBeginPlay
  (Variables|Default|SetbCanAct false)
  (Utilities|FlowControl|Delay 3.0)
  (Variables|Default|SetbCanAct true)
  (Variables|Default|SetTargetPlayer (Game|GetPlayerCharacter 0))
  (Utilities|Time|SetTimerbyEvent (delegate Custom|TryAttackPlayer) (Variables|Default|GetAttackCheckInterval) true))

(event Collision|EventActorBeginOverlap
  (params (OtherActor :type Actor%20Object%20Reference)))

(event EventTick
  (params (DeltaSeconds :type Float%20%28single-precision%29)))

(event Game|Damage|EventAnyDamage
  (params (Damage :type Float%20%28single-precision%29) (DamageType :type Damage%20Type%20Object%20Reference) (InstigatedBy :type Controller%20Object%20Reference) (DamageCauser :type Actor%20Object%20Reference))
  (Class|BossBase|ApplyBossDamage Damage (Variables|Default|GetBasicAttackPostureDamage)))

(event EventOnBossStunned
  (Variables|Default|SetbIsAttacking false)
  (Variables|Default|SetbIsComboPattern false)
  (Animation|StopAnimMontage 0)
  (Development|PrintString "BOSS STUNNED!"))

(event EventOnBossStunEnded
  (Development|PrintString "BOSS STUN END"))

(event EventOnBossDead
  (Variables|Default|SetbIsAttacking false)
  (Variables|Default|SetbIsComboPattern false)
  (Animation|StopAnimMontage 0)
  (Development|PrintString "BOSS Dead!")
  (bind _asbp_player_character (Utilities|Casting|CastToBP_PlayerCharacter (Game|GetPlayerCharacter 0)))
  (Default|ShowBattleResult _asbp_player_character "BOSS DEFEATED"))

(fn ConstructionScript)

(fn HandleBossAttackStart
  (bind _returnvalue (Transformation|GetActorLocation))
  (bind _returnvalue_2 (Math|Vector|MakeVector 0.0 0.0 6e+01))
  (bind _targetplayer (Variables|Default|GetTargetPlayer))
  (bind _returnvalue_3 (+ _returnvalue _returnvalue_2))
  (if (not (Variables|Default|GetbIsDead))
    (if (not (Variables|Default|GetbIsStunned))
      (Development|PrintString "BP HandleBossAttackStart")
      (bind _outhit (Collision|SphereTraceForObjects _returnvalue_3 (+ _returnvalue_3 (* (Transformation|GetActorForwardVector) (Variables|Default|GetBossAttackTraceDistance))) (Variables|Default|GetBossAttackTraceRadius) (Utilities|Array|MakeArray "ObjectTypeQuery3") false (Utilities|Array|MakeArray self) "ForDuration"))
      (if true
        (Development|PrintString (Utilities|String|ToString(Text) (Utilities|Text|FormatText "Boss Trace Hit Actor: {HitActorName}" (Utilities|GetDisplayName (.HitActor (Collision|BreakHitResult _outhit))))))
        (Utilities|IsValid (.HitActor (Collision|BreakHitResult _outhit))
          (:Is%20Valid
            (if (== (.HitActor (Collision|BreakHitResult _outhit)) _targetplayer)
              (Game|Damage|ApplyDamage _targetplayer (Variables|Default|GetBossAttackDamage) (Pawn|GetController) self)
              (Development|PrintString "Boss Hit Player")
              (else
                (Development|PrintString "Boss Hit Actor But Not TargetPlayer"))))
          (:Is%20Not%20Valid
            (Development|PrintString "Boss Trace Hit But Actor Is Invalid")))
        (else
          (Development|PrintString "Boss Attack Missed"))))))

(fn HandleBossAttackEnd
  (Development|PrintString "BP HandleBossAttackEnd")
  (if (Variables|Default|GetbIsComboPattern)
    (Development|PrintString "Combo pattern continues")
    (else
      (Variables|Default|SetbIsAttacking false)
      (Development|PrintString "Boss Attack End"))))

(fn SelectAttackPattern
  (switch int (Math|Random|RandomIntegerinRange 0 2)
    (:0
      (return "NewEnumerator0"))
    (:1
      (return "NewEnumerator1"))
    (:2
      (return "NewEnumerator2"))))