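; Stage manager for a boss-rush run that sequences fights, tracks win or loss, and grants upgrades between stages.
; BeginPlay caches player and boss and builds the upgrade pool; later stages respawn a boss by index and reset the player.
; Boss defeat shows random upgrade choices in a widget; ApplyUpgrade routes picks to Stat or Combat components.
; Run clear only prints, RestartCurrentStage is a stub, and choice removal re-rolls its index, allowing duplicates.
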(event Custom|StartStage
  (params (StageIndex :type Integer))
  (bind _playercharacter (Variables|References|GetPlayerCharacter))
  (Variables|Stage|SetbStageCleared false)
  (Variables|Stage|SetbStageRunning true)
  (bind _output_get (Variables|Stage|SetCurrentStageIndex StageIndex))
  (Development|PrintString (Utilities|String|ToString(Text) (Utilities|Text|FormatText "Stage Start: {StageIndex}" _output_get)))
  (if (> (Variables|Stage|GetCurrentStageIndex) 1)
    (Utilities|IsValid (Variables|References|GetCurrentBoss)
      (:Is%20Valid
        (Actor|DestroyActor (Variables|References|GetCurrentBoss))
        (bind _returnvalue (Game|SpawnActorfromClass (Utilities|Array|Get(acopy) (Variables|Default|GetBossClasses) (- (Variables|Stage|GetCurrentStageIndex) 1)) (Variables|Default|GetBossSpawnTransform) "Undefined" "MultiplyWithRoot" 0 0))
        (bind _output_get_2 (Variables|References|SetCurrentBoss _returnvalue))
        (Variables|/Game/Blueprints/Player/BP_PlayerCharacter.BP_PlayerCharacter_C|SetBossRef (Variables|References|GetPlayerCharacter) _output_get_2)
        (Class|BossBase|ResetBossState _output_get_2)
        (Pawn|SpawnDefaultController _output_get_2)
        (Development|PrintString "Boss Spawned")
        (Utilities|FlowControl|Delay 0.2)
        (CallFunction|SetBossLookatPlayer)
        (Utilities|IsValid _playercharacter
          (:Is%20Valid
            (Transformation|SetActorTransform _playercharacter (Variables|Default|GetPlayerStartTransform))
            (Components|Movement|StopMovementImmediately (Variables|/Script/Engine.Character|GetCharacterMovement _playercharacter))
            (Class|PlayerCombatComponent|ResetCombatState (Variables|/Script/BossRush.BossRushCharacter|GetCombatComponent _playercharacter))))))))

(event Custom|OnBossDefeated
  (if (not (Variables|Stage|GetbStageCleared))
    (Variables|Stage|SetbStageCleared true)
    (Variables|Stage|SetbStageRunning false)
    (Development|PrintString "Stage Clear!")
    (CallFunction|ShowUpgradeSelection)))

(event Custom|ShowUpgradeSelection
  (bind _returnvalue (Game|GetPlayerController 0))
  (Development|PrintString "Show Upgrade Selection")
  (CallFunction|GenerateUpgradeChoices 3)
  (bind _returnvalue_2 (UserInterface|CreateWidget (Variables|Default|GetUpgradeSelectWidgetClass) (Game|GetPlayerController 0)))
  (bind _output_get (Variables|Default|SetUpgradeSelectWidgetRef _returnvalue_2))
  (Default|SetupChoices _output_get (Variables|Upgrade|GetCurrentUpgradeChoices) self)
  (UserInterface|Viewport|AddtoViewport (Variables|Default|GetUpgradeSelectWidgetRef) 0)
  (Variables|/Script/Engine.PlayerController|SetbShowMouseCursor _returnvalue true)
  (Input|SetInputModeUIOnly _returnvalue (Variables|Default|GetUpgradeSelectWidgetRef) "DoNotLock" false))

(event Custom|StartNextStage
  (Variables|Stage|SetCurrentStageIndex (+ (Variables|Stage|GetCurrentStageIndex) 1))
  (if (> (Variables|Stage|GetCurrentStageIndex) (Variables|Stage|GetMaxStageCount))
    (Development|PrintString "Run Clear!")
    (else
      (Development|PrintString "Start Next Stage")
      (Class|PlayerStatComponent|RestoreAllStats (Variables|/Script/BossRush.BossRushCharacter|GetStatComponent (Variables|References|GetPlayerCharacter)))
      (CallFunction|StartStage (Variables|Stage|GetCurrentStageIndex)))))

(event Custom|OnPlayerDefeated
  (if (Variables|Stage|GetbStageRunning)
    (Variables|Stage|SetbStageRunning false)
    (Development|PrintString "Player Defeated")
    (Default|ShowBattleResult (Variables|References|GetPlayerCharacter) "YOU DIED")))

(event Custom|RestartCurrentStage
  (Development|PrintString "Restart Current Stage"))

(event Custom|InitializeUpgradeList
  (Utilities|Array|Clear (Variables|Upgrade|GetAllUpgrades))
  (Utilities|Array|Add (Variables|Upgrade|GetAllUpgrades) (Utilities|Struct|MakeUpgradeData "AttackPowerUp" "공격력 강화" "공격력이 5 증가합니다." "IncreaseAttackPower" 5.0))
  (Utilities|Array|Add (Variables|Upgrade|GetAllUpgrades) (Utilities|Struct|MakeUpgradeData "MaxHPUp" "생명력 강화" "최대 체력이 25 증가합니다." "IncreaseMaxHP" 25.0))
  (Utilities|Array|Add (Variables|Upgrade|GetAllUpgrades) (Utilities|Struct|MakeUpgradeData "MaxStaminaUp" "스태미나 강화" "최대 스태미나가 25 증가합니다." "IncreaseMaxStamina" 25.0))
  (Utilities|Array|Add (Variables|Upgrade|GetAllUpgrades) (Utilities|Struct|MakeUpgradeData "StaminaRegenUp" "호흡 안정" "스태미나 회복 속도가 5 증가합니다." "IncreaseStaminaRegen" 5.0))
  (Utilities|Array|Add (Variables|Upgrade|GetAllUpgrades) (Utilities|Struct|MakeUpgradeData "DodgeCostDown" "가벼운 발걸음" "회피 스태미나 소모량이 5 감소합니다." "ReduceDodgeCost" 5.0))
  (Utilities|Array|Add (Variables|Upgrade|GetAllUpgrades) (Utilities|Struct|MakeUpgradeData "ParryPostureUp" "정확한 반격" "패링 성공 시 보스 자세 피해가 10 증가합니다." "IncreaseParryPostureDamage" 1e+01))
  (Development|PrintString (Utilities|String|ToString(Text) (Utilities|Text|FormatText "Upgrade List Initialized: {length}" (Utilities|Array|Length (Variables|Upgrade|GetAllUpgrades))))))

(event EventBeginPlay
  (bind _asbp_player_character (Utilities|Casting|CastToBP_PlayerCharacter (Game|GetPlayerCharacter 0)))
  (bind _output_get (Variables|References|SetPlayerCharacter _asbp_player_character))
  (Development|PrintString "StageManager: Player Cached")
  (Variables|Default|SetPlayerStartTransform (Transformation|GetActorTransform _output_get))
  (bind _returnvalue (Actor|GetActorOfClass "/Script/BossRush.BossBase"))
  (bind _output_get_2 (Variables|References|SetCurrentBoss _returnvalue))
  (Development|PrintString "StageManager: Boss Cached")
  (Variables|Default|SetBossSpawnTransform "")
  (CallFunction|InitializeUpgradeList)
  (CallFunction|StartStage (Variables|Stage|GetCurrentStageIndex)))

(event Collision|EventActorBeginOverlap
  (params (OtherActor :type Actor%20Object%20Reference)))

(event EventTick
  (params (DeltaSeconds :type Float%20%28single-precision%29)))

(fn ConstructionScript)

(fn GenerateUpgradeChoices
  (params (ChoiceCount :type Integer))
  (Utilities|Array|Clear (Variables|Upgrade|GetCurrentUpgradeChoices))
  (LocalVariables|SetTempUpgradePool (Variables|Upgrade|GetAllUpgrades))
  (for _index (range 0 (- ChoiceCount 1))
    (if (> (Utilities|Array|Length (LocalVariables|GetTempUpgradePool)) 0)
      (Utilities|Array|Add (Variables|Upgrade|GetCurrentUpgradeChoices) (Utilities|Array|Get(acopy) (LocalVariables|GetTempUpgradePool) (Math|Random|RandomIntegerinRange 0 (- (Utilities|Array|Length (LocalVariables|GetTempUpgradePool)) 1))))
      (Utilities|Array|RemoveIndex (LocalVariables|GetTempUpgradePool) (Math|Random|RandomIntegerinRange 0 (- (Utilities|Array|Length (LocalVariables|GetTempUpgradePool)) 1)))))
  (Development|PrintString "Upgrade Choices Generated")
  (for _array_element (Variables|Upgrade|GetCurrentUpgradeChoices)
    (Development|PrintString (Utilities|String|ToString(Text) (.DisplayName (Utilities|Struct|BreakUpgradeData _array_element))))))

(fn ApplyUpgrade
  (params (UpgradeData :type Upgrade%20Data%20Structure))
  (bind (_upgradeid _displayname _description _upgradetype _value) (Utilities|Struct|BreakUpgradeData UpgradeData))
  (Utilities|Array|Add (Variables|Upgrade|GetSelectedUpgrades) UpgradeData)
  (Development|PrintString (Utilities|String|ToString(Text) (Utilities|Text|FormatText "Selected Upgrade: {DisplayName}" _displayname)))
  (switch Utilities|FlowControl|Switch|SwitchonEUpgradeType _upgradetype
    (:IncreaseAttackPower
      (Development|PrintString (Utilities|String|ToString(Text) (Utilities|Text|FormatText "Apply Attack Power Upgrade / Value: {val}" _value)))
      (Class|PlayerCombatComponent|AddAttackDamage (Variables|/Script/BossRush.BossRushCharacter|GetCombatComponent (Variables|References|GetPlayerCharacter)) _value)
      (CallFunction|PrintSelectedUpgrades))
    (:IncreaseMaxHP
      (Development|PrintString (Utilities|String|ToString(Text) (Utilities|Text|FormatText "Apply Max HP Upgrade / Value: {val}" _value)))
      (Class|PlayerStatComponent|AddMaxHP (Variables|/Script/BossRush.BossRushCharacter|GetStatComponent (Variables|References|GetPlayerCharacter)) _value)
      (CallFunction|PrintSelectedUpgrades))
    (:IncreaseMaxStamina
      (Development|PrintString (Utilities|String|ToString(Text) (Utilities|Text|FormatText "Apply Max Stamina Upgrade / Value: {val}" _value)))
      (Class|PlayerStatComponent|AddMaxStamina (Variables|/Script/BossRush.BossRushCharacter|GetStatComponent (Variables|References|GetPlayerCharacter)) _value)
      (CallFunction|PrintSelectedUpgrades))
    (:IncreaseStaminaRegen
      (Development|PrintString (Utilities|String|ToString(Text) (Utilities|Text|FormatText "Apply Stamina Regen Upgrade / Value: {val}" _value)))
      (Class|PlayerStatComponent|AddStaminaRegen (Variables|/Script/BossRush.BossRushCharacter|GetStatComponent (Variables|References|GetPlayerCharacter)) _value)
      (CallFunction|PrintSelectedUpgrades))
    (:ReduceDodgeCost
      (Development|PrintString (Utilities|String|ToString(Text) (Utilities|Text|FormatText "Apply Dodge Cost Upgrade / Value: {val}" _value)))
      (Class|PlayerCombatComponent|ReduceDodgeStaminaCost (Variables|/Script/BossRush.BossRushCharacter|GetCombatComponent (Variables|References|GetPlayerCharacter)) _value)
      (CallFunction|PrintSelectedUpgrades))
    (:IncreaseParryPostureDamage
      (Development|PrintString (Utilities|String|ToString(Text) (Utilities|Text|FormatText "Apply Parry Posture Upgrade / Value: {val}" _value)))
      (Class|PlayerCombatComponent|AddPlayerParryPostureDamage (Variables|/Script/BossRush.BossRushCharacter|GetCombatComponent (Variables|References|GetPlayerCharacter)) _value)
      (CallFunction|PrintSelectedUpgrades))))

(fn PrintSelectedUpgrades
  (for (_array_element _array_index) (Variables|Upgrade|GetSelectedUpgrades)
    (Development|PrintText (Utilities|Text|FormatText "{Index}. {Name}" (+ _array_index 1) (.DisplayName (Utilities|Struct|BreakUpgradeData _array_element))))))

(fn SetBossLookatPlayer
  (bind _currentboss (Variables|References|GetCurrentBoss))
  (bind _currentboss_2 (Variables|References|GetCurrentBoss))
  (bind _playercharacter (Variables|References|GetPlayerCharacter))
  (bind _returnvalue (Pawn|GetController _currentboss))
  (bind _returnvalue_2 (Transformation|GetActorLocation _currentboss_2))
  (bind _returnvalue_3 (Transformation|GetActorLocation _playercharacter))
  (bind _returnvalue_4 (Math|Rotator|FindLookatRotation _returnvalue_2 _returnvalue_3))
  (bind _yaw (Math|Rotator|BreakRotator _returnvalue_4))
  (bind _returnvalue_5 (Math|Rotator|MakeRotator 0.0 0.0 _yaw))
  (Utilities|IsValid (Variables|References|GetCurrentBoss)
    (:Is%20Valid
      (Utilities|IsValid (Variables|References|GetPlayerCharacter)
        (:Is%20Valid
          (Transformation|SetActorRotation (Variables|References|GetCurrentBoss) _returnvalue_5)
          (Utilities|IsValid _returnvalue
            (:Is%20Valid
              (Pawn|SetControlRotation _returnvalue _returnvalue_5))))))))