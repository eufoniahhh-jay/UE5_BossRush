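; Player character Blueprint for boss combat that owns the combat HUD and handles incoming damage.
; On BeginPlay it creates the HUD and caches the first BP_BossDummy in the level.
; Tick polls StatComponent and the boss to push player HP, stamina and boss HP into the HUD.
; AnyDamage checks CombatComponent for invincibility, then an open parry window (both only print), before passing damage to StatComponent.
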(event EventBeginPlay
  (bind _returnvalue (UserInterface|CreateWidget (Variables|Default|GetCombatHUDClass) (Game|GetPlayerController 0)))
  (bind _output_get (Variables|Default|SetCombatHUD _returnvalue))
  (UserInterface|Viewport|AddtoViewport _output_get 0)
  (bind _outactors (Actor|GetAllActorsOfClass "/Game/Blueprints/Boss/BP_BossDummy.BP_BossDummy_C"))
  (bind _asbp_boss_dummy (Utilities|Casting|CastToBP_BossDummy (Utilities|Array|Get(acopy) _outactors)))
  (Variables|Default|SetBossDummyRef _asbp_boss_dummy))

(event Collision|EventActorBeginOverlap
  (params (OtherActor :type Actor%20Object%20Reference)))

(event EventTick
  (params (DeltaSeconds :type Float%20%28single-precision%29))
  (bind _statcomponent (Variables|Default|GetStatComponent))
  (bind _bossdummyref (Variables|Default|GetBossDummyRef))
  (Utilities|IsValid (Variables|Default|GetCombatHUD)
    (:Is%20Valid
      (Utilities|IsValid (Variables|Default|GetBossDummyRef)
        (:Is%20Valid
          (Default|UpdateHUD (Variables|Default|GetCombatHUD) (Class|PlayerStatComponent|GetCurrentHP _statcomponent) (Class|PlayerStatComponent|GetMaxHP _statcomponent) (Class|PlayerStatComponent|GetCurrentStamina _statcomponent) (Class|PlayerStatComponent|GetMaxStamina _statcomponent) (Variables|/Game/Blueprints/Boss/BP_BossDummy.BP_BossDummy_C|GetCurrentHP _bossdummyref) (Variables|/Game/Blueprints/Boss/BP_BossDummy.BP_BossDummy_C|GetMaxHP _bossdummyref)))))))

(event Game|Damage|EventAnyDamage
  (params (Damage :type Float%20%28single-precision%29) (DamageType :type Damage%20Type%20Object%20Reference) (InstigatedBy :type Controller%20Object%20Reference) (DamageCauser :type Actor%20Object%20Reference))
  (if (Class|PlayerCombatComponent|IsInvincible (Variables|Default|GetCombatComponent))
    (Development|PrintString "Damage ignored: Invincible")
    (elif (Class|PlayerCombatComponent|IsParryWindowOpen (Variables|Default|GetCombatComponent))
      (Development|PrintString "Parry Success")
      (else
        (Class|PlayerStatComponent|TakeDamage (Variables|Default|GetStatComponent) Damage)))))

(fn ConstructionScript)